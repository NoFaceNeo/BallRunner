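; BP_Crystal is a crystal actor that flies to the player and vanishes when overlapped, like a pickup.
; Any actor overlap starts two timelines: one pulls it toward player pawn 0's live location, the other shrinks it to zero scale.
; Both lerp from the current transform each update, so changes compound, and whichever timeline finishes first destroys the actor.
; No score or inventory logic is present.
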(event EventBeginPlay)

(event EventTick
  (params (DeltaSeconds :type Float%20%28single-precision%29)))

(event Collision|EventActorBeginOverlap
  (params (OtherActor :type Actor%20Object%20Reference))
  (Utilities|FlowControl|Sequence
    (:then_0
      (bind _crystallerp (Timeline|CrystalVa Play)
        (:Update
          (Transformation|SetActorLocation (Math|Vector|Lerp(Vector) (Transformation|GetActorLocation) (Transformation|GetActorLocation (Game|Player|GetPlayerPawn 0)) _crystallerp) false false))
        (:Finished
          (Actor|DestroyActor :!label _label))))
    (:then_1
      (bind _crystalscale (Timeline|CrystalScale PlayFromStart)
        (:Update
          (Transformation|SetActorRelativeScale3D (Math|Vector|Lerp(Vector) (Transformation|GetActorScale3D) "0, 0, 0" _crystalscale)))
        (:Finished
          (goto _label))))))

(fn ConstructionScript)